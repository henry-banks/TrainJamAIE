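; Obstacle Blueprint that destroys the player's twin-stick ship when it is hit.
; On Hit, it casts the other actor to TwinStickPawn, spawns an explosion effect at that actor's transform, then disables the pawn's tick and hides its ship mesh instead of destroying it.
; The construction script applies a configurable mesh and material to its static mesh from the RefMesh and RefMaterial variables.
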(event EventBeginPlay)

(event EventTick
  (params (DeltaSeconds :type Float%20%28single-precision%29)))

(event Collision|EventActorBeginOverlap
  (params (OtherActor :type Actor%20Object%20Reference)))

(event Collision|EventHit
  (params (MyComp :type Primitive%20Component%20Object%20Reference) (Other :type Actor%20Object%20Reference) (OtherComp :type Primitive%20Component%20Object%20Reference) (bSelfMoved :type Boolean) (HitLocation :type Vector :default "0, 0, 0") (HitNormal :type Vector :default "0, 0, 0") (NormalImpulse :type Vector :default "0, 0, 0") (Hit :type Hit%20Result%20Structure%20%28by%20ref%29))
  (bind _astwin_stick_pawn (Utilities|Casting|CastToTwinStickPawn Other))
  (Game|SpawnActorfromClass "/Game/StarterContent/Blueprints/Blueprint_Effect_Explosion.Blueprint_Effect_Explosion_C" (Transformation|GetActorTransform Other) "Undefined" 0 _astwin_stick_pawn)
  (Actor|Tick|SetActorTickEnabled _astwin_stick_pawn)
  (Rendering|SetVisibility (Variables|/Game/TwinStickBP/Blueprints/TwinStickPawn.TwinStickPawn_C|GetShipMeshComponent _astwin_stick_pawn) false false))

(fn ConstructionScript
  (bind _staticmesh (Variables|Default|GetStaticMesh))
  (Components|StaticMesh|SetStaticMesh _staticmesh (Variables|Default|GetrefMesh))
  (Rendering|Material|SetMaterial _staticmesh 0 (Variables|Default|GetrefMaterial)))